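; RoadGen is a construction-script spline road generator that builds road and optional left and right guardrails from spline mesh components.
; It syncs a per-point data array to the spline point count, padding with defaults or trimming.
; Each segment takes bank, width, thickness and guardrail flags from its start point's entry, optionally closing the loop.
; Optional text labels show point indices above the road; the collision setting is unwired.
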(event EventBeginPlay)

(event Collision|EventActorBeginOverlap
  (params (OtherActor :type Actor%20Object%20Reference)))

(event EventTick
  (params (DeltaSeconds :type Float%20%28single-precision%29)))

(fn ConstructionScript
  (Utilities|FlowControl|Sequence
    (:then_0
      (|StorenumberofSplinepoints))
    (:then_1
      (|Buildroaddataarray))
    (:then_2
      (|ConsturctionLoop)
      (|StoreDrawLeftRightLightPosts)
      (Utilities|FlowControl|Sequence
        (:then_0
          (CallFunction|BuildRoadElement (Variables|Default|GetCurrentLoopIndex) (Variables|Default|GetRoadMesh)))
        (:then_1
          (if (Variables|Default|GetDrawLeftGaurdRail)
            (CallFunction|BuildRoadElement (Variables|Default|GetCurrentLoopIndex) (Variables|Default|GetLeftGaurdRail))))
        (:then_2
          (if (Variables|Default|GetDrawRightGaurdRail)
            (CallFunction|BuildRoadElement (Variables|Default|GetCurrentLoopIndex) (Variables|Default|GetRightGaurdRail))))))
    (:then_3
      (|DrawRoadText))))

(fn BuildRoadElement
  (params (LoopIndex :type Integer) (RoadElementMesh :type Static%20Mesh%20Object%20Reference))
  (LocalVariables|SetLocal_CurrentLoopIndex LoopIndex)
  (LocalVariables|SetLocal_NextLoopIndex (Math|Integer|%(Integer) (+ LoopIndex 1) (Variables|Default|GetNumber%20of%20spline%20points)))
  (LocalVariables|SetLocal_RoadelementMash RoadElementMesh)
  (Utilities|FlowControl|Sequence
    (:then_0
      (LocalVariables|SetLocal_StartLocation (.LocalLocation (Class|SplineComponent|GetLocalLocationandTangentatSplinePoint (Variables|Default|GetSpline) (LocalVariables|GetLocal_CurrentLoopIndex))))
      (LocalVariables|SetLocal_StartTangent (.LocalTangent (Class|SplineComponent|GetLocalLocationandTangentatSplinePoint (Variables|Default|GetSpline) (LocalVariables|GetLocal_CurrentLoopIndex))))
      (LocalVariables|SetLocal_EndLocation (.LocalLocation (Class|SplineComponent|GetLocalLocationandTangentatSplinePoint (Variables|Default|GetSpline) (LocalVariables|GetLocal_NextLoopIndex))))
      (LocalVariables|SetLocal_EndTangent (.LocalTangent (Class|SplineComponent|GetLocalLocationandTangentatSplinePoint (Variables|Default|GetSpline) (LocalVariables|GetLocal_NextLoopIndex))))
      (LocalVariables|SetLocal_StartRoll (.roadbank (Utilities|Array|Get(acopy) (Variables|Default|GetRoadDataArray) (LocalVariables|GetLocal_CurrentLoopIndex))))
      (LocalVariables|SetLocal_StartScale (Math|Vector2D|MakeVector2D (.roadwidth (Utilities|Array|Get(acopy) (Variables|Default|GetRoadDataArray) (LocalVariables|GetLocal_CurrentLoopIndex))) (.roadthickness (Utilities|Array|Get(acopy) (Variables|Default|GetRoadDataArray) (LocalVariables|GetLocal_CurrentLoopIndex)))))
      (LocalVariables|SetLocal_EndRoll (.roadbank (Utilities|Array|Get(acopy) (Variables|Default|GetRoadDataArray) (LocalVariables|GetLocal_CurrentLoopIndex))))
      (LocalVariables|SetLocal_EndScale (Math|Vector2D|MakeVector2D (.roadwidth (Utilities|Array|Get(acopy) (Variables|Default|GetRoadDataArray) (LocalVariables|GetLocal_CurrentLoopIndex))) (.roadthickness (Utilities|Array|Get(acopy) (Variables|Default|GetRoadDataArray) (LocalVariables|GetLocal_CurrentLoopIndex))))))
    (:then_1
      (bind _returnvalue (AddComponent|AddSplineMeshComponent false))
      (LocalVariables|SetLocal_CurrentSplineMesh _returnvalue)
      (Components|StaticMesh|SetStaticMesh (LocalVariables|GetLocal_CurrentSplineMesh) (LocalVariables|GetLocal_RoadelementMash))
      (SplineMesh|SetStartandEnd (LocalVariables|GetLocal_CurrentSplineMesh) (LocalVariables|GetLocal_StartLocation) (LocalVariables|GetLocal_StartTangent) (LocalVariables|GetLocal_EndLocation) (LocalVariables|GetLocal_EndTangent) :!class /Script/Engine.SplineMeshComponent)
      (Class|SplineMeshComponent|SetStartRoll (LocalVariables|GetLocal_CurrentSplineMesh) (LocalVariables|GetLocal_StartRoll))
      (Class|SplineMeshComponent|SetEndRoll (LocalVariables|GetLocal_CurrentSplineMesh) (LocalVariables|GetLocal_EndRoll))
      (SplineMesh|SetStartScale (LocalVariables|GetLocal_CurrentSplineMesh) (LocalVariables|GetLocal_StartScale) :!class /Script/Engine.SplineMeshComponent)
      (SplineMesh|SetEndScale (LocalVariables|GetLocal_CurrentSplineMesh) (LocalVariables|GetLocal_EndScale) :!class /Script/Engine.SplineMeshComponent))))